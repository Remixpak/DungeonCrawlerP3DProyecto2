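; BP_SpikeTrap is an interactable trap that damages the player character when it touches the trap's box.
; Interact flips the Active flag and switches the Box collision off or on to match, and CanInteract always allows it.
; On Box overlap, a BP_ThirdPersonCharacter receives DamageAmount through its BPCHealthSystemComponent, and a debug message prints.
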(event `/Game/BPI_Interactable.Interact`
  (params (Actor :type "Actor Object Reference"))
  (if (`self.bActive`)
    (set `self.bActive` false)
    (`PrimitiveComponent.SetCollisionEnabled` (`self.Box`) "NoCollision")
    (else
      (set `self.bActive` true)
      (`PrimitiveComponent.SetCollisionEnabled` (`self.Box`) "QueryAndPhysics"))))

(event `self.Box.OnComponentBeginOverlap`
  (params (OverlappedComponent :type "PrimitiveComponent Object Reference") (OtherActor :type "Actor Object Reference") (OtherComp :type "PrimitiveComponent Object Reference") (OtherBodyIndex :type Integer) (bFromSweep :type Boolean) (SweepResult :type "HitResult Structure (by ref)"))
  (bind _asbp_third_person_character (cast `/Game/ThirdPerson/Blueprints/BP_ThirdPersonCharacter` OtherActor))
  (`HealthSystemComponent.ReceiveDamage` (`/Game/ThirdPerson/Blueprints/BP_ThirdPersonCharacter.BPC_HealthSystemComponent` _asbp_third_person_character) (`self.DamageAmount`))
  (`KismetSystemLibrary.PrintString` "oh me dañaste"))

(fn `CanInteract`
  (params (Actor :type "Actor Object Reference"))
  (returns (CanInteract :type Boolean))
  (return true))

(fn `UserConstructionScript`)