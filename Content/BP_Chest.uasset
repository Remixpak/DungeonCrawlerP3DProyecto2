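; BP_Chest is a one-time interactable chest that gives coins to the player character.
; CanInteract allows interaction only while the Opened flag is false.
; Interact sets Opened, then casts the interacting actor to BP_ThirdPersonCharacter, adds CoinsToGive coins and switches the Box material to gold.
; Opened is set before the cast, so any interacting actor marks the chest opened, even without a payout.
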(event `/Game/BPI_Interactable.Interact`
  (params (Actor :type "Actor Object Reference"))
  (set `self.bOpened` true)
  (bind _asbp_third_person_character (cast `/Game/ThirdPerson/Blueprints/BP_ThirdPersonCharacter` Actor))
  (`/Game/ThirdPerson/Blueprints/BP_ThirdPersonCharacter.AddCoins` _asbp_third_person_character (`self.CoinsToGive`))
  (`PrimitiveComponent.SetMaterial` (`self.Box`) 0 "/Game/StarterContent/Materials/M_Metal_Gold.M_Metal_Gold"))

(fn `CanInteract`
  (params (Actor :type "Actor Object Reference"))
  (returns (CanInteract :type Boolean))
  (if (`self.bOpened`)
    (return false)
    (else
      (return true))))

(fn `UserConstructionScript`)