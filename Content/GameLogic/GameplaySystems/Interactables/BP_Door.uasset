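; BP_Door is an interactable door that uses a lock component to gate opening.
; Interact passes the actor to BP_LockComponent's TryUnlock, and its OnUnlocked event alternately plays and reverses a timeline that rotates the door mesh's yaw.
; On BeginPlay, a dynamic material instance tints the mesh red, blue or green to match the lock's key color.
; Actor overlap only prints a debug string.
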(event `self.ReceiveBeginPlay`
  (bind _doormaterial (`self.DoorMaterial`))
  (add `/Game/GameLogic/GameplaySystems/UnlockDoorsSystem/BP_LockComponent.OnUnlocked` (`self.GetComponentByClass` "/Game/GameLogic/GameplaySystems/UnlockDoorsSystem/BP_LockComponent.BP_LockComponent_C") (delegate `Handled_OnUnlocked`))
  (bind _returnvalue (`PrimitiveComponent.CreateDynamicMaterialInstance` (`self.DoorMesh`) 0 "/Game/Assets/Shaders/M_Dynamic.M_Dynamic" "None"))
  (`PrimitiveComponent.SetMaterial` (`self.DoorMesh`) 0 _returnvalue)
  (set `self.DoorMaterial` _returnvalue)
  (switch `/Game/GameLogic/Enums/E_KeyColor` (`/Game/GameLogic/GameplaySystems/UnlockDoorsSystem/BP_LockComponent.KeyColor` (`self.BP_LockComponent`))
    (:`NewEnumerator0`
      (`MaterialInstanceDynamic.SetVectorParameterValue` _doormaterial "BaseColor" (struct :`R` 1.0 :`G` 0.039766 :`A` 1.0)))
    (:`NewEnumerator1`
      (`MaterialInstanceDynamic.SetVectorParameterValue` _doormaterial "BaseColor" (struct :`G` 0.046939 :`B` 1.0 :`A` 1.0)))
    (:`NewEnumerator2`
      (`MaterialInstanceDynamic.SetVectorParameterValue` _doormaterial "BaseColor" (struct :`G` 1.0 :`B` 0.090115 :`A` 1.0)))))

(event `Handled_OnUnlocked`
  (params (Instigator :type "Actor Object Reference"))
  (`/Engine/EditorBlueprintResources/StandardMacros.FlipFlop`
    (:`A`
      (bind (_direction _rotationvalue) (`Timeline|OpenTimeline` :!via `PlayFromStart` :!label _label)
        (:`Update`
          (`SceneComponent.K2_SetRelativeRotation` (`self.DoorMesh`) (`KismetMathLibrary.MakeRotator` 0.0 0.0 _rotationvalue) false false))))
    (:`B`
      (goto _label :!via `Reverse`))))

(event `self.ReceiveActorBeginOverlap`
  (params (OtherActor :type "Actor Object Reference"))
  (`KismetSystemLibrary.PrintString` "Hello"))

(event `/Game/GameLogic/Interfaces/BPI_Interactable.Interact`
  (params (Actor :type "Actor Object Reference"))
  (`/Game/GameLogic/GameplaySystems/UnlockDoorsSystem/BP_LockComponent.TryUnlock` (`self.GetComponentByClass` "/Game/GameLogic/GameplaySystems/UnlockDoorsSystem/BP_LockComponent.BP_LockComponent_C") Actor))

(fn `CanInteract`
  (params (Actor :type "Actor Object Reference"))
  (returns (CanInteract :type Boolean))
  (return true))

(fn `UserConstructionScript`)