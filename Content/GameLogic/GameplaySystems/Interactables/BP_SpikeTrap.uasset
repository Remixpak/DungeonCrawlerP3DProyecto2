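; BP_SpikeTrap is an interactable spike trap that damages the player character when it is active.
; Interact toggles the Active flag and switches the Box collision on or off, and CanInteract always allows it.
; While active, a Box overlap by BP_ThirdPersonCharacter sends DamageAmount to that character's health system component.
; Debug prints in Spanish report toggling and hits.
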(event `/Game/GameLogic/Interfaces/BPI_Interactable.Interact`
  (params (Actor :type "Actor Object Reference"))
  (bind _box (`self.Box`))
  (if (`self.bActive`)
    (`PrimitiveComponent.SetCollisionEnabled` _box "NoCollision")
    (set `self.bActive` false)
    (`KismetSystemLibrary.PrintString` "Se desactivo la trampa" true true (struct :`G` 1.0 :`B` 0.138169 :`A` 1.0))
    (else
      (`PrimitiveComponent.SetCollisionEnabled` _box "QueryAndPhysics")
      (set `self.bActive` true)
      (`KismetSystemLibrary.PrintString` "Se activo la trampa" true true (struct :`G` 1.0 :`B` 0.080409 :`A` 1.0)))))

(event `self.Box.OnComponentBeginOverlap`
  (params (OverlappedComponent :type "PrimitiveComponent Object Reference") (OtherActor :type "Actor Object Reference") (OtherComp :type "PrimitiveComponent Object Reference") (OtherBodyIndex :type Integer) (bFromSweep :type Boolean) (SweepResult :type "HitResult Structure (by ref)"))
  (if (`self.bActive`)
    (bind _asbp_third_person_character (cast `/Game/ThirdPerson/Blueprints/BP_ThirdPersonCharacter` OtherActor))
    (`HealthSystemComponent.ReceiveDamage` (`/Game/ThirdPerson/Blueprints/BP_ThirdPersonCharacter.BPC_HealthSystemComponent` _asbp_third_person_character) (`self.DamageAmount`))
    (`KismetSystemLibrary.PrintString` "oh me dañaste")))

(fn `CanInteract`
  (params (Actor :type "Actor Object Reference"))
  (returns (CanInteract :type Boolean))
  (return true))

(fn `UserConstructionScript`)