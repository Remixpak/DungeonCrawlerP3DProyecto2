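; Health system component that triggers a dungeon game restart when health is depleted.
; On BeginPlay it binds a handler to its OnDamageReceived dispatcher.
; The handler prints MaxHealth and, if it is zero or below, calls RestartGame on BP_GM_Dungeon and prints a Spanish player-death message.
; The graph only reads MaxHealth; it does not apply damage itself.
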(event `self.ReceiveBeginPlay`
  ; Damage Logic
  (add `self.OnDamageReceived` (delegate `OnDamageReceived_Event`)))

(event `OnDamageReceived_Event`
  (bind _maxhealth (`self.MaxHealth`))
  ; Damage Logic
  (`KismetSystemLibrary.PrintString` (`KismetStringLibrary.Conv_DoubleToString` _maxhealth))
  (if (<= _maxhealth 0.0)
    (bind _asbp_gm_dungeon (cast `/Game/GameLogic/Core/BP_GM_Dungeon` (`GameplayStatics.GetGameMode`)))
    (`/Game/GameLogic/Core/BP_GM_Dungeon.RestartGame` _asbp_gm_dungeon)
    (`KismetSystemLibrary.PrintString` "Jugador a muerto" true true (struct :`R` 1.0 :`B` 0.072545 :`A` 1.0))))