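; Actor component for the drop system that awards a coin reward to the player.
; DropCoins uses the AlreadyDropped flag to pay out only once, adding its Coins value to CurrentPlayerCoins on BP_GM_Core.
; The coins are credited directly through the game mode with no pickup spawned, and the new total is printed on screen.
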(event `DropCoins`
  (if (not (`self.AlreadyDropped?`))
    (set `self.AlreadyDropped?` true)
    (bind _asbp_gm_core (cast `/Game/GameLogic/Core/BP_GM_Core` (`GameplayStatics.GetGameMode`)))
    (bind _output_get (set `/Game/GameLogic/Core/BP_GM_Core.CurrentPlayerCoins` (+ (`/Game/GameLogic/Core/BP_GM_Core.CurrentPlayerCoins` _asbp_gm_core) (`self.Coins`)) _asbp_gm_core))
    (`KismetSystemLibrary.PrintString` (`KismetStringLibrary.Conv_IntToString` _output_get) true true (struct :`R` 1.0 :`G` 0.027013 :`A` 1.0))))