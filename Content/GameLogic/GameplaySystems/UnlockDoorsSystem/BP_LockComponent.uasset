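; BP_LockComponent is a lock component in the door-unlock system that gates an interaction behind a key of a given color.
; TryUnlock returns true when not blocked; otherwise it asks the interactor's BP_KeyInventoryComponent for a key matching KeyColor.
; A match fires OnUnlocked and returns true without clearing Blocked in that function, while a miss returns false; both print a debug string.
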(fn `TryUnlock`
  (params (Interactor :type "Actor Object Reference"))
  (returns (ReturnValue :type Boolean))
  ; Try Unlock function
  (if (`self.Blocked`)
    (if (`/Game/GameLogic/GameplaySystems/UnlockDoorsSystem/BP_KeyInventoryComponent.HasKey` (`Actor.GetComponentByClass` Interactor "/Game/GameLogic/GameplaySystems/UnlockDoorsSystem/BP_KeyInventoryComponent.BP_KeyInventoryComponent_C") (`self.KeyColor`))
      (`KismetSystemLibrary.PrintString` "La tiene")
      (`self.OnUnlocked` null)
      (return true)
      (else
        (`KismetSystemLibrary.PrintString` "No La tiene")
        (return false)))
    (else
      (return true))))