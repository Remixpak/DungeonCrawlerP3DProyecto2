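; Dungeon game mode blueprint that tracks the player's score toward a goal and can restart the level.
; AddScore adds to the current points and prints the total, or a win message once the goal is reached.
; On reaching the goal it casts the player character to BP_MainCharacter and changes its color using the M_TableRound material.
; RestartGame reloads the current level by name.
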(event `AddScore`
  (params (ScoreToAdd :type Integer))
  (bind _output_get (set `self.CurrentPoints` (+ (`self.CurrentPoints`) ScoreToAdd)))
  (bind _returnvalue (`KismetStringLibrary.Conv_IntToString` _output_get))
  (bind _returnvalue_2 (>= _output_get (`self.GoalPoints`)))
  (`KismetSystemLibrary.PrintString` (select `bool` _returnvalue_2 :`false` _returnvalue :`true` (`KismetStringLibrary.Concat_StrStr` "Has Ganado con: " _returnvalue)))
  (if _returnvalue_2
    (bind _asbp_main_character (cast `/Game/GameLogic/Core/BP_MainCharacter` (`GameplayStatics.GetPlayerCharacter` 0)))
    (`/Game/GameLogic/Core/BP_MainCharacter.ChangeColor` _asbp_main_character "/Game/StarterContent/Props/Materials/M_TableRound.M_TableRound")))

(event `RestartGame`
  (bind _returnvalue (`GameplayStatics.GetCurrentLevelName` true))
  (`GameplayStatics.OpenLevel` (`KismetStringLibrary.Conv_StringToName` _returnvalue)))

(fn `UserConstructionScript`)